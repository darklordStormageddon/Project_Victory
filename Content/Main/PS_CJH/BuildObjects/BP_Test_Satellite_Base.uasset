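; Base satellite actor that assembles itself from parts, spins slowly at random, and can be captured by a player spaceship.
; On BeginPlay a server-to-multicast call places scene slots from a DataTable and attaches random body, panel and attachment actors plus fixed connector types.
; Connectors are linked to their part and the satellite, and a bound event broadcasts body detachment.
; Sphere overlap captures it, and Tick pulls it toward the ship's gravity point, scaled by ship speed.
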(event `Set Scene Transform`
  ;[1 1 1] 컴포넌트 지정된 위치에 랜덤종류 스폰
  (bind _returnvalue (`|GetDataTableRow` (`self.Location_DataTable`) "Component")
    (:`then`
      (bind (_body_transform _panel_transform _attachment_transform _connector1_transform _connector2_transform) (break `/Game/Main/PS_KSM/Sattelites/DS_Location` _returnvalue))
      (`SceneComponent.K2_SetRelativeTransform` (`self.SceneChild1`) (`|GetArrayItem` _connector1_transform) false false)
      (`SceneComponent.K2_SetRelativeTransform` (`self.SceneChild2`) (`|GetArrayItem` _connector1_transform 1) false false)
      (`SceneComponent.K2_SetRelativeTransform` (`self.SceneChild3`) (`|GetArrayItem` _connector2_transform) false false)
      (`SceneComponent.K2_SetRelativeTransform` (`self.SceneChild4`) (`|GetArrayItem` _connector2_transform 1) false false)
      (`SceneComponent.K2_SetRelativeTransform` (`self.SceneChild5`) (`|GetArrayItem` _panel_transform) false false)
      (`SceneComponent.K2_SetRelativeTransform` (`self.SceneChild6`) (`|GetArrayItem` _panel_transform 1) false false)
      (`SceneComponent.K2_SetRelativeTransform` (`self.SceneChild7`) (`|GetArrayItem` _attachment_transform) false false)
      (`SceneComponent.K2_SetRelativeTransform` (`self.SceneChild8`) (`|GetArrayItem` _attachment_transform 1) false false))))

(event `self.ReceiveBeginPlay`
  (`self.Server_Set_Satellite`)
  (set `self.Rotation` (* (`KismetMathLibrary.RandomUnitVector`) 0.3)))

(event `Server_Set_Satellite`
  (`self.Multi_Set_Satellite`))

(event `Multi_Set_Satellite`
  (bind _connector_types (`self.Connector_Types`))
  (bind _connector1 (`self.Connector1`))
  (bind _connector2 (`self.Connector2`))
  (bind _connector3 (`self.Connector3`))
  (bind _connector4 (`self.Connector4`))
  (bind _outitem (`KismetArrayLibrary.Array_Random` (`self.PanelTypes`)))
  (bind _outitem_2 (`KismetArrayLibrary.Array_Random` (`self.Attachment_Types`)))
  (bind _output (`|GetArrayItem` _connector_types))
  (bind _output_2 (`|GetArrayItem` _connector_types 1))
  ;[1 1 1] scene child component 순서는 connector 1~4, panel 1~2, attachment 1~2
  (`self.Set Scene Transform`)
  (bind _actor (`self.Spawn& Attach` (`KismetArrayLibrary.Array_Random` (`self.BodyTypes`)) (`self.SceneRoot`)))
  (bind _asbody_base (cast `BodyBase` _actor))
  (set `self.Body` _asbody_base)
  (bind _actor_2 (`self.Spawn& Attach` _output (`self.SceneChild1`)))
  (bind _asbp_connector (cast `/Game/Main/PS_KSM/Sattelites/BP_Connector` _actor_2))
  (set `self.Connector1` _asbp_connector)
  (bind _actor_3 (`self.Spawn& Attach` _output (`self.SceneChild2`)))
  (bind _asbp_connector_2 (cast `/Game/Main/PS_KSM/Sattelites/BP_Connector` _actor_3))
  (set `self.Connector2` _asbp_connector_2)
  (bind _actor_4 (`self.Spawn& Attach` _output_2 (`self.SceneChild3`)))
  (bind _asbp_connector_2 (cast `/Game/Main/PS_KSM/Sattelites/BP_Connector2` _actor_4))
  (set `self.Connector3` _asbp_connector_2)
  (bind _actor_5 (`self.Spawn& Attach` _output_2 (`self.SceneChild4`)))
  (bind _asbp_connector_2_2 (cast `/Game/Main/PS_KSM/Sattelites/BP_Connector2` _actor_5))
  (set `self.Connector4` _asbp_connector_2_2)
  (bind _actor_6 (`self.Spawn& Attach` _outitem (`self.SceneChild5`)))
  (bind _aspanel_base (cast `PanelBase` _actor_6))
  (set `self.Panel1` _aspanel_base)
  (bind _actor_7 (`self.Spawn& Attach` _outitem (`self.SceneChild6`)))
  (bind _aspanel_base_2 (cast `PanelBase` _actor_7))
  (set `self.Panel2` _aspanel_base_2)
  (bind _actor_8 (`self.Spawn& Attach` _outitem_2 (`self.SceneChild7`)))
  (bind _asattachment_base (cast `Attachment_Base` _actor_8))
  (set `self.Attachment1` _asattachment_base)
  (bind _actor_9 (`self.Spawn& Attach` _outitem_2 (`self.SceneChild8`)))
  (bind _asattachment_base_2 (cast `Attachment_Base` _actor_9))
  (set `self.Attachment2` _asattachment_base_2)
  (set `/Game/Main/PS_KSM/Sattelites/BP_Connector.Attachment` (`self.Attachment1`) _connector1)
  (set `/Game/Main/PS_KSM/Sattelites/BP_Connector.Attachment` (`self.Attachment2`) _connector2)
  (set `/Game/Main/PS_KSM/Sattelites/BP_Connector2.Panel` (`self.Panel2`) _connector3)
  (set `/Game/Main/PS_KSM/Sattelites/BP_Connector2.Panel` (`self.Panel1`) _connector4)
  (set `Connector_Base.Attached_Satellite` self _connector1)
  (set `Connector_Base.Attached_Satellite` self _connector2)
  (set `Connector_Base.Attached_Satellite` self _connector3)
  (set `Connector_Base.Attached_Satellite` self _connector4)
  (add `self.CanDestroyBody` (delegate `Enable Body Physics`)))

(event `Enable Body Physics`
  ;[1 1 1] scene child component 순서는 connector 1~4, panel 1~2, attachment 1~2
  (`BodyBase.Broadcast_Body_Detachment` (`self.Body`)))

(event `self.Sphere.OnComponentBeginOverlap`
  (params (OverlappedComponent :type "PrimitiveComponent Object Reference") (OtherActor :type "Actor Object Reference") (OtherComp :type "PrimitiveComponent Object Reference") (OtherBodyIndex :type Integer) (bFromSweep :type Boolean) (SweepResult :type "HitResult Structure (by ref)"))
  (bind _asmy_psj_spaceship (cast `/Game/Main/PS_PSJ/Blueprint/Spaceship/MyPSJ_Spaceship` OtherActor))
  (bind _output_get (set `self.As My PSJ Spaceship` _asmy_psj_spaceship))
  (set `self.bIsCaptured` true)
  (set `/Game/Main/PS_PSJ/Blueprint/Spaceship/MyPSJ_Spaceship.Captured_Satellite` self _output_get))

(event `self.ReceiveTick`
  (params (DeltaSeconds :type "Float (single-precision)"))
  (bind _returnvalue (`self.K2_GetActorLocation`))
  (bind (_rotation_x _rotation_y _rotation_z) (`KismetMathLibrary.BreakVector` (`self.Rotation`)))
  (bind _as_my_psj_spaceship (`self.As My PSJ Spaceship`))
  (`self.K2_AddActorWorldRotation` (`KismetMathLibrary.MakeRotator` _rotation_x _rotation_y _rotation_z))
  (if (`self.bIsCaptured`)
    (bind _gf_location (`/Game/Main/PS_PSJ/Blueprint/Spaceship/MyPSJ_Spaceship.GetGravityLocation` _as_my_psj_spaceship))
    (bind _returnvalue_2 (- _gf_location _returnvalue))
    (if (not (<= (`KismetMathLibrary.VSize` _returnvalue_2) 30.0))
      (`self.K2_SetActorLocation` (+ (* (* _returnvalue_2 0.001) (`KismetMathLibrary.VSize` (`self.GetVelocity` _as_my_psj_spaceship))) _returnvalue) true))))

(fn `OnRep_Connector_Destruct_Count`)

(fn `Spawn& Attach`
  (params (ActorClass :type "Actor Class Reference") (Scene :type "SceneComponent Object Reference"))
  (returns (Actor :type "Actor Object Reference"))
  (bind _returnvalue (`|SpawnActorFromClass` ActorClass (`SceneComponent.K2_GetComponentToWorld` Scene) "AlwaysSpawn" "MultiplyWithRoot" null null))
  (`self.K2_AttachToComponent` _returnvalue Scene "None" "SnapToTarget" "SnapToTarget" "SnapToTarget" false)
  (return _returnvalue))

(fn `UserConstructionScript`)