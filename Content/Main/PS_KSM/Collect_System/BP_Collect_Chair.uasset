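; BP_Collect_Chair is an interactable chair that hands player control over to the BP_Collect_Panel in the level.
; The panel reference is looked up on BeginPlay, and sphere overlap by BP_Player toggles the chair's input and a WBP_Temp message widget.
; Pressing Enter stores the player pawn as the panel's PrePlayer, enables the panel's input, possesses it and removes the message.
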(event `self.ReceiveBeginPlay`
  (bind _returnvalue (`GameplayStatics.GetActorOfClass` "/Game/Main/PS_KSM/Collect_System/BP_Collect_Panel.BP_Collect_Panel_C"))
  (set `self.BP_Collect_Panel` _returnvalue))

(event `self.Sphere.OnComponentBeginOverlap`
  (params (OverlappedComponent :type "PrimitiveComponent Object Reference") (OtherActor :type "Actor Object Reference") (OtherComp :type "PrimitiveComponent Object Reference") (OtherBodyIndex :type Integer) (bFromSweep :type Boolean) (SweepResult :type "HitResult Structure (by ref)"))
  (cast `/Game/Main/PS_KSM/BP_Player` OtherActor)
  (`self.EnableInput` (`GameplayStatics.GetPlayerController` 0))
  (bind _returnvalue (`|CreateWidget` "/Game/Main/PS_KSM/Collect_System/WBP_Temp.WBP_Temp_C"))
  (bind _output_get (set `self.Message Widget` _returnvalue))
  (`UserWidget.AddToViewport` _output_get 0))

(event `self.Sphere.OnComponentEndOverlap`
  (params (OverlappedComponent :type "PrimitiveComponent Object Reference") (OtherActor :type "Actor Object Reference") (OtherComp :type "PrimitiveComponent Object Reference") (OtherBodyIndex :type Integer))
  (bind _message_widget (`self.Message Widget`))
  (cast `/Game/Main/PS_KSM/BP_Player` OtherActor)
  (`self.DisableInput` (`GameplayStatics.GetPlayerController` 0))
  (`/Engine/EditorBlueprintResources/StandardMacros.IsValid` _message_widget
    (:`Is Valid`
      (`Widget.RemoveFromParent` _message_widget))))

(event `Key|Enter`
  (params (Key :type "Key Structure"))
  (bind _returnvalue (`GameplayStatics.GetPlayerController` 0))
  (bind _message_widget (`self.Message Widget`))
  (bind _bp_collect_panel (`self.BP_Collect_Panel`))
  (:`Pressed`
    (bind _asbp_player (cast `/Game/Main/PS_KSM/BP_Player` (`Controller.K2_GetPawn` _returnvalue)))
    (set `/Game/Main/PS_KSM/Collect_System/BP_Collect_Panel.Pre_Player` _asbp_player _bp_collect_panel)
    (`self.EnableInput` _bp_collect_panel _returnvalue)
    (`Controller.Possess` _returnvalue _bp_collect_panel)
    (`/Engine/EditorBlueprintResources/StandardMacros.IsValid` _message_widget
      (:`Is Valid`
        (`Widget.RemoveFromParent` _message_widget)))))

(fn `UserConstructionScript`)