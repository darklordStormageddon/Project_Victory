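; Possessable collection station where a player deploys and aims a vacuum, laser or drill to dismantle objects and gather ore.
; Tool switching runs server events that chain timeline-driven hatch and tool movements.
; The vacuum pulls a sphere-traced, highlighted target with distance-attenuated force and collects nearby ore, the laser line-traces to damage connectors, and the cabled drill damages parts on overlap.
; Multicasts drive laser and vacuum Niagara effects; exiting repossesses the previous pawn.
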(event `self.ReceiveBeginPlay`
  (`self.SetOwner` (`GameplayStatics.GetPlayerController` 0))
  (`KismetSystemLibrary.K2_SetTimer` null "Clear_Target" 2.0 true)
  (`ActorComponent.Deactivate` (`self.NS_Laser1`))
  (`ActorComponent.Deactivate` (`self.NS_Spiral`))
  (add `self.ToolIsOut` (delegate `After Tool Is Out`))
  (add `self.ToolIsIn` (delegate `After Tool Is In`))
  (`NiagaraComponent.SetVariableVec3` (`self.NS_Laser1`) "Beam End" (`SceneComponent.K2_GetComponentLocation` (`self.L_Scene`))))

(event `After Tool Is In`
  ;[1 1 1] 서버만
  (`self.Server_Tool_In`))

(event `After Tool Is Out`
  ;[1 1 1] 서버만
  (`self.Server_Tool_Out`))

(event `Server_Tool_In`
  ;[1 1 1] 서버만
  (set `self.bIsToolOut` false)
  (set `self.bIsGettingToolOut` false)
  (`KismetSystemLibrary.Delay` 0.5)
  (`SceneComponent.K2_SetWorldLocation` (`self.PreTool`) (`SceneComponent.K2_GetComponentLocation` (`self.Init_Scene`)) false false)
  (set `self.PreTool` null))

(event `Server_Tool_Out`
  ;[1 1 1] 서버만
  (set `self.bIsGettingToolOut` false)
  (set `self.bIsToolOut` true)
  (switch `E_COLLECT_TOOL_TYPE` (`self._Tool_Type`)
    (:`Vacuum`
      (set `self.PreTool` (`self.V_Base`)))
    (:`Laser`
      (set `self.PreTool` (`self.L_Base`)))
    (:`Drill`
      (set `self.PreTool` (`self.D_Base`)))
    (:`NONE`
      (set `self.PreTool` null))))

(event `Pull Tool Out`
  (params (`Static Mesh` :type "StaticMeshComponent Object Reference"))
  ;[1 1 1] 도구 꺼내기 파이프라인
  (`self.Move_Center` `Static Mesh`)
  (`self.Open_Box`)
  (`KismetSystemLibrary.Delay` 0.2)
  (`self.Tool_Out` `Static Mesh`)
  (`KismetSystemLibrary.Delay` 0.2)
  (`self.Close_Box`)
  (`KismetSystemLibrary.Delay` 0.2)
  (`self.ToolIsOut`))

(event `Push Tool In`
  (params (`Static Mesh` :type "StaticMeshComponent Object Reference"))
  ;[1 1 1] 도구 넣기 파이프라인
  (`self.Open_Box`)
  (`KismetSystemLibrary.Delay` 0.2)
  (`self.Tool_In` `Static Mesh`)
  (`KismetSystemLibrary.Delay` 0.2)
  (`self.Close_Box`)
  (`KismetSystemLibrary.Delay` 0.2)
  (`self.ToolIsIn`))

(event `Tool_Out`
  (params (`Static Mesh` :type "StaticMeshComponent Object Reference"))
  ;[1 1 1] 도구 꺼내기
  (bind (_direction _up) (`Timeline|Timeline` :!via `PlayFromStart`)
    (:`Update`
      (`SceneComponent.K2_SetWorldLocation` `Static Mesh` (`KismetMathLibrary.VLerp` (`SceneComponent.K2_GetComponentLocation` (`self.Set_Scene`)) (`SceneComponent.K2_GetComponentLocation` (`self.Spawn_Scene`)) _up) false false))))

(event `Move_Center`
  (params (`Static Mesh` :type "StaticMeshComponent Object Reference"))
  ;[1 1 1] 가운데로 도구 세팅
  (`SceneComponent.K2_SetWorldLocation` `Static Mesh` (`SceneComponent.K2_GetComponentLocation` (`self.Set_Scene`)) false false))

(event `Tool_In`
  (params (`Static Mesh` :type "StaticMeshComponent Object Reference"))
  ;[1 1 1] 도구 넣기
  (bind (_direction _up) (`Timeline|Timeline_1` :!via `PlayFromStart`)
    (:`Update`
      (`SceneComponent.K2_SetWorldLocation` `Static Mesh` (`KismetMathLibrary.VLerp` (`SceneComponent.K2_GetComponentLocation` (`self.Spawn_Scene`)) (`SceneComponent.K2_GetComponentLocation` (`self.Set_Scene`)) _up) false false))))

(event `Open_Box`
  ;[1 1 1] 박스 열기
  (bind (_direction _hatch) (`Timeline|Open Hatch` :!via `PlayFromStart`)
    (:`Update`
      (`SceneComponent.K2_SetWorldLocation` (`self.Center_L`) (`KismetMathLibrary.VLerp` (`SceneComponent.K2_GetComponentLocation` (`self.Center_L_Scene`)) (`SceneComponent.K2_GetComponentLocation` (`self.Middle_L`)) _hatch) false false)
      (`SceneComponent.K2_SetWorldLocation` (`self.Center_R`) (`KismetMathLibrary.VLerp` (`SceneComponent.K2_GetComponentLocation` (`self.Center_R_Scene`)) (`SceneComponent.K2_GetComponentLocation` (`self.Middle_R`)) _hatch) false false))))

(event `EnhancedInput|/Game/Main/PS_KSM/Collect_System/Collect_Input/IA_Unpossess`
  (params (ActionValue :type Boolean) (ElapsedSeconds :type "Float (double-precision)") (TriggeredSeconds :type "Float (double-precision)") (InputAction :type "InputAction Object Reference" :default "/Game/Main/PS_KSM/Collect_System/Collect_Input/IA_Unpossess.IA_Unpossess"))
  ;[1 1 1] 자리 떠나기
  (:`Triggered`
    (`Widget.RemoveFromParent` (`self.Wbp_CollectPanel`))
    (`Controller.Possess` (`GameplayStatics.GetPlayerController` 0) (`self.Pre_Player`))))

(event `EnhancedInput|/Game/Main/PS_KSM/Collect_System/Collect_Input/IA_Laser`
  (params (ActionValue :type Boolean) (ElapsedSeconds :type "Float (double-precision)") (TriggeredSeconds :type "Float (double-precision)") (InputAction :type "InputAction Object Reference" :default "/Game/Main/PS_KSM/Collect_System/Collect_Input/IA_Laser.IA_Laser"))
  ;[1 1 1] 레이저 꺼내기
  (:`Triggered`
    (`self.Server_Pull_Laser`)))

(event `Close_Box`
  ;[1 1 1] 박스 닫기
  (bind (_direction _hatch) (`Timeline|Timeline_0` :!via `PlayFromStart`)
    (:`Update`
      (`SceneComponent.K2_SetWorldLocation` (`self.Center_L`) (`KismetMathLibrary.VLerp` (`SceneComponent.K2_GetComponentLocation` (`self.Middle_L`)) (`SceneComponent.K2_GetComponentLocation` (`self.Center_L_Scene`)) _hatch) false false)
      (`SceneComponent.K2_SetWorldLocation` (`self.Center_R`) (`KismetMathLibrary.VLerp` (`SceneComponent.K2_GetComponentLocation` (`self.Middle_R`)) (`SceneComponent.K2_GetComponentLocation` (`self.Center_R_Scene`)) _hatch) false false))))

(event `Server_Pull_Laser`
  ;[1 1 1] 레이저 꺼내기
  (if (`self.bIsGettingToolOut`)
    _
    (elif (`self.bIsToolOut`)
      (if (== (`self.PreTool`) (`self.L_Base`))
        (set `self.bIsGettingToolOut` true)
        (`self.Push Tool In` (`self.L_Base`))
        (`self.Server_Deactivate_Laser`)
        (else
          (set `self.bIsGettingToolOut` true)
          (`self.Push Tool In` (`self.PreTool`))
          (`KismetSystemLibrary.Delay` 0.6)
          (`self.Pull Tool Out` (`self.L_Base`) :!label _label)
          (set `self._Tool_Type` "Laser")))
      (else
        (set `self.bIsGettingToolOut` true)
        (goto _label)))))

(event `EnhancedInput|/Game/Main/PS_KSM/Collect_System/Collect_Input/IA_Drill`
  (params (ActionValue :type Boolean) (ElapsedSeconds :type "Float (double-precision)") (TriggeredSeconds :type "Float (double-precision)") (InputAction :type "InputAction Object Reference" :default "/Game/Main/PS_KSM/Collect_System/Collect_Input/IA_Drill.IA_Drill"))
  ;[1 1 1] 드릴 꺼내기
  (:`Triggered`
    (`self.Server_Pull_Drill`)))

(event `Server_Pull_Drill`
  ;[1 1 1] 드릴 꺼내기
  (if (`self.bIsGettingToolOut`)
    _
    (elif (`self.bIsToolOut`)
      (if (== (`self.PreTool`) (`self.D_Base`))
        (set `self.bIsGettingToolOut` true)
        (`self.Push Tool In` (`self.D_Base`))
        (else
          (set `self.bIsGettingToolOut` true)
          (`self.Push Tool In` (`self.PreTool`))
          (`KismetSystemLibrary.Delay` 0.6)
          (`self.Pull Tool Out` (`self.D_Base`) :!label _label_2)
          (set `self._Tool_Type` "Drill")))
      (else
        (set `self.bIsGettingToolOut` true)
        (goto _label_2)))))

(event `EnhancedInput|/Game/Main/PS_KSM/Collect_System/Collect_Input/IA_Vacuum`
  (params (ActionValue :type Boolean) (ElapsedSeconds :type "Float (double-precision)") (TriggeredSeconds :type "Float (double-precision)") (InputAction :type "InputAction Object Reference" :default "/Game/Main/PS_KSM/Collect_System/Collect_Input/IA_Vacuum.IA_Vacuum"))
  ;[1 1 1] 흡입기 꺼내기
  (:`Triggered`
    (`self.Server_Pull_Vacuum`)))

(event `Client_RestoreControl`
  (params (TargetPawn :type "Pawn Object Reference")))

(event `Server_ExitSeat`
  (bind _pre_player (`self.Pre_Player`))
  ;[1 1 1] PSJ_RPC 때문에 추가하거나 수정한 부분
  (`Controller.Possess` (`self.GetController`) _pre_player)
  (bind _asmy_psj_character (cast `/Game/Main/PS_PSJ/Blueprint/PlayerCharacter/MyPSJ_Character` _pre_player))
  (`/Game/Main/PS_PSJ/Blueprint/PlayerCharacter/MyPSJ_Character.Client_WakeUp_Input` _asmy_psj_character))

(event `Server_Pull_Vacuum`
  ;[1 1 1] 흡입기 꺼내기
  (if (`self.bIsGettingToolOut`)
    _
    (elif (`self.bIsToolOut`)
      (if (== (`self.PreTool`) (`self.V_Base`))
        (set `self.bIsGettingToolOut` true)
        (`self.Push Tool In` (`self.V_Base`))
        (`self.Server_Deactivate_Vacuum`)
        (else
          (set `self.bIsGettingToolOut` true)
          (`self.Push Tool In` (`self.PreTool`))
          (`KismetSystemLibrary.Delay` 0.6)
          (`self.Pull Tool Out` (`self.V_Base`) :!label _label_3)
          (set `self._Tool_Type` "Vacuum")))
      (else
        (set `self.bIsGettingToolOut` true)
        (goto _label_3)))))

(event `self.ReceivePossessed`
  (params (NewController :type "Controller Object Reference"))
  ;[1 1 1] PSJ_RPC 때문에 추가하거나 수정한 부분
  (`self.Client_Init_Input` NewController))

(event `EnhancedInput|/Game/Main/PS_KSM/Collect_System/Collect_Input/IA_Unpossess`
  (params (ActionValue :type Boolean) (ElapsedSeconds :type "Float (double-precision)") (TriggeredSeconds :type "Float (double-precision)") (InputAction :type "InputAction Object Reference" :default "/Game/Main/PS_KSM/Collect_System/Collect_Input/IA_Unpossess.IA_Unpossess"))
  ;[1 1 1] PSJ_RPC 때문에 추가하거나 수정한 부분
  (:`Started`
    (`self.Server_ExitSeat`)))

(event `Client_Init_Input`
  (params (NewParam :type "Controller Object Reference"))
  ;[1 1 1] PSJ_RPC 때문에 추가하거나 수정한 부분
  (bind _asplayer_controller (cast `PlayerController` NewParam))
  (bind _returnvalue (pcsubsystem `EnhancedInputLocalPlayerSubsystem` _asplayer_controller))
  (`EnhancedInputSubsystemInterface.ClearAllMappings` _returnvalue)
  (`EnhancedInputSubsystemInterface.AddMappingContext` _returnvalue "/Game/Main/PS_KSM/Collect_System/Collect_Input/IMC_Collect.IMC_Collect" 0 (struct))
  (`self.EnableInput` _asplayer_controller)
  (bind _returnvalue_2 (`|CreateWidget` "/Game/Main/PS_JHS/Blueprint/UI/Panel/WBP_UIPanelCollectSeat.WBP_UIPanelCollectSeat_C"))
  (bind _output_get (set `self.Wbp_CollectPanel` _returnvalue_2))
  (`UserWidget.AddToViewport` _output_get 0))

(event `Trace_Ore`
  (bind _collect_target (`self.Collect_Target`))
  (bind _returnvalue (`SceneComponent.K2_GetComponentLocation` (`self.V_Scene`)))
  (bind _returnvalue_2 (+ _returnvalue (* (`KismetMathLibrary.Normal` (`SceneComponent.GetForwardVector` (`self.V_Scene`))) 3000.0)))
  ;[1 1 1] Sphere Trace로 광물 타겟 지정 및 하이라이트 + 종류 표시
  (set `self.Spiral End` _returnvalue_2)
  (bind _outhit (`KismetSystemLibrary.SphereTraceSingle` _returnvalue _returnvalue_2 20.0 "TraceTypeQuery1"))
  (`/Engine/EditorBlueprintResources/StandardMacros.IsValid` (`.HitActor` (`GameplayStatics.BreakHitResult` _outhit))
    (:`Is Valid`
      (bind _asbp_collectable_base (cast `/Game/Main/PS_KSM/Collect_System/Collectables/BP_Collectable_Base` (`.HitActor` (`GameplayStatics.BreakHitResult` _outhit))))
      (`/Engine/EditorBlueprintResources/StandardMacros.IsValid` _collect_target
        (:`Is Valid`
          (if (not (== _collect_target _asbp_collectable_base))
            (`/Game/Main/PS_KSM/Collect_System/Collectables/BP_Collectable_Base.Deselect` (`self.Collect_Target`))
            (bind _output_get (set `self.Collect_Target` _asbp_collectable_base))
            (`/Game/Main/PS_KSM/Collect_System/Collectables/BP_Collectable_Base.Highlight Selected` _output_get)
            (`PrimitiveComponent.SetPhysicsLinearVelocity` (`Collectable_base.Mesh` _output_get) (0.0 0.0 0.0) false "None")))
        (:`Is Not Valid`
          (bind _output_get_2 (set `self.Collect_Target` _asbp_collectable_base))
          (`/Game/Main/PS_KSM/Collect_System/Collectables/BP_Collectable_Base.Highlight Selected` _output_get_2))))))

(event `Satellite_Trace`
  (bind _d_scene (`self.D_Scene`))
  (bind _returnvalue (`SceneComponent.K2_GetComponentLocation` _d_scene))
  ;[1 1 1] 드릴 발사 위치
  (`KismetSystemLibrary.LineTraceSingle` _returnvalue (+ _returnvalue (* (`KismetMathLibrary.Normal` (`SceneComponent.GetForwardVector` _d_scene)) 5000.0)) "TraceTypeQuery1"))

(event `EnhancedInput|/Game/Main/PS_KSM/GameSettings/Input/IA_Look`
  (params (ActionValue :type "Vector2D Structure") (ElapsedSeconds :type "Float (double-precision)") (TriggeredSeconds :type "Float (double-precision)") (InputAction :type "InputAction Object Reference" :default "/Game/Main/PS_KSM/GameSettings/Input/IA_Look.IA_Look"))
  (:`Triggered`
    (switch `E_COLLECT_TOOL_TYPE` (`self._Tool_Type`)
      (:`Vacuum`
        (`self.Rotate Turret(Clamp)` (`self.V_Holder`) (`self.V_Turret`) ActionValue_X ActionValue_Y))
      (:`Laser`
        (`self.Rotate Turret(Clamp)` (`self.L_Holder`) (`self.L_Turret`) ActionValue_X ActionValue_Y))
      (:`Drill`
        (`self.Rotate Turret(Clamp)` (`self.D_Holder`) (`self.D_Turret`) ActionValue_X ActionValue_Y)))))

(event `Rotate Turret(Clamp)`
  (params (Holder :type "StaticMeshComponent Object Reference") (Turret :type "StaticMeshComponent Object Reference") (`X Value` :type "Float (double-precision)") (`Y Value` :type "Float (double-precision)"))
  (bind _returnvalue (* `X Value` -1.0))
  (bind _returnvalue_2 (* `Y Value` -1.0))
  (bind _relativerotation_roll (`KismetMathLibrary.BreakRotator` (`SceneComponent.RelativeRotation` Turret)))
  (bind (_relativerotation_roll_2 _relativerotation_pitch _relativerotation_yaw) (`KismetMathLibrary.BreakRotator` (`SceneComponent.RelativeRotation` Holder)))
  (if (<= (`KismetMathLibrary.Abs` (+ _relativerotation_yaw _returnvalue)) 50.0)
    (`SceneComponent.K2_AddLocalRotation` Holder (`KismetMathLibrary.MakeRotator` 0.0 0.0 _returnvalue) false false)
    (if (<= (`KismetMathLibrary.Abs` (+ _relativerotation_roll _returnvalue_2)) 50.0)
      (`SceneComponent.K2_AddLocalRotation` Turret (`KismetMathLibrary.MakeRotator` _returnvalue_2) false false))))

(event `Rotate_Drill`
  ;[1 1 1] 드릴 회전
  (if (`|EnumEquality` (`self._Tool_Type`) "Drill")
    (`SceneComponent.K2_AddLocalRotation` (`self.D_Drill`) (`KismetMathLibrary.MakeRotator` 0.0 0.0 (* (stale `self.ReceiveTick` DeltaSeconds) 500.0)) false false)))

(event `self.ReceiveTick`
  (params (DeltaSeconds :type "Float (single-precision)"))
  ;[1 1 1] 드릴 회전
  (`|ExecutionSequence`
    (:`then_0`
      (`self.Server_Trace_Ore`))
    (:`then_1`
      (`self.Server_Collect_Ore`))))

(event `Server_Trace_Ore`
  ;[1 1 1] 드릴 회전
  (if (`|EnumEquality` (`self._Tool_Type`) "Vacuum")
    (`self.Trace_Ore`)))

(event `Clear_Target`
  (bind _collect_target (`self.Collect_Target`))
  ;[1 1 1] 타겟 초기화(주기적으로 타이머로 호출)
  (if (not (`self.bIsCollecting`))
    (`/Engine/EditorBlueprintResources/StandardMacros.IsValid` _collect_target
      (:`Is Valid`
        (if (> (`KismetMathLibrary.VSize` (- (`self.K2_GetActorLocation` _collect_target) (`self.K2_GetActorLocation`))) 600.0)
          (`/Game/Main/PS_KSM/Collect_System/Collectables/BP_Collectable_Base.Deselect` _collect_target)
          (set `self.Collect_Target` null))))))

(event `Server_Collect_Ore`
  ;[1 1 1] 드릴 회전
  ;;[1 1 1] 수거
  (if (`self.bVacuum`)
    (set `self.bIsCollecting` true)
    (bind _outactors (`GameplayStatics.GetAllActorsOfClass` "/Game/Main/PS_KSM/Collect_System/Collectables/BP_Collectable_Base.BP_Collectable_Base_C"))
    (for _array_element _outactors
      (if (<= (`KismetMathLibrary.VSize` (- (`self.K2_GetActorLocation` _array_element) (`self.K2_GetActorLocation`))) 800.0)
        (bind _asbp_collectable_base (cast `/Game/Main/PS_KSM/Collect_System/Collectables/BP_Collectable_Base` _array_element))
        (`/Game/Main/PS_KSM/Collect_System/Collectables/BP_Collectable_Base.Collect_Ore` _asbp_collectable_base)
        (`self.K2_DestroyActor` _asbp_collectable_base)))
    (set `self.bIsCollecting` false)))

(event `Server_Activate_Laser`
  ;[1 1 1] RPC
  (`self.Multi_Activate_Laser`))

(event `Server_Set_Beam_End`
  (params (Location :type "Vector Structure"))
  ;[1 1 1] RPC
  (`self.Multi_Set_Beam_End` Location))

(event `EnhancedInput|/Game/Main/PS_KSM/GameSettings/Input/IA_Interact`
  (params (ActionValue :type Boolean) (ElapsedSeconds :type "Float (double-precision)") (TriggeredSeconds :type "Float (double-precision)") (InputAction :type "InputAction Object Reference" :default "/Game/Main/PS_KSM/GameSettings/Input/IA_Interact.IA_Interact"))
  (bind __tool_type (`self._Tool_Type`))
  ;[1 1 1] 분리 작업
  (:`Triggered`
    (if (`self.bIsToolOut`)
      (`self.UpdateDurabilityAndDamage`)
      (switch `E_COLLECT_TOOL_TYPE` __tool_type
        (:`Vacuum`
          ;[1 1 1] 흡입
          (`self.Vacuum_On_Server`))
        (:`Laser`
          (`self.Server_Laser_On`))
        (:`Drill`
          ;[1 1 1] 드릴 데미지
          (`self.Drill_On_Server`)))))
  (:`Completed`
    (switch `E_COLLECT_TOOL_TYPE` __tool_type
      (:`Vacuum`
        (`self.Vacuum_Off_Server`))
      (:`Laser`
        (`self.Server_Deactivate_Laser`)))))

(event `Server_Laser_On`
  (bind _returnvalue (`SceneComponent.K2_GetComponentLocation` (`self.L_Scene`)))
  (bind _returnvalue_2 (`SceneComponent.GetForwardVector` (`self.L_Scene`)))
  ;[1 1 1] 분리 작업
  (bind _outhit (`KismetSystemLibrary.LineTraceSingle` _returnvalue (+ _returnvalue (* _returnvalue_2 2000.0)) "TraceTypeQuery1"))
  (if (`GameplayStatics.BreakHitResult` _outhit)
    (`self.Server_Set_Beam_End` (`.Location` (`GameplayStatics.BreakHitResult` _outhit)))
    (else
      (`self.Server_Set_Beam_End` (+ (`SceneComponent.K2_GetComponentLocation` (`self.L_Scene`)) (* _returnvalue_2 20000.0)))))
  (`self.Multi_Activate_Laser`)
  (bind _asconnector_base (cast `Connector_Base` (`.HitActor` (`GameplayStatics.BreakHitResult` _outhit))))
  (`Connector_Base.Damage_Connector` _asconnector_base (* (`.Time` (`GameplayStatics.BreakHitResult` _outhit)) (`self._OutToolDamage`))))

(event `Multi_Activate_Laser`
  ;[1 1 1] RPC
  (`ActorComponent.Activate` (`self.NS_Laser1`) false))

(event `Multi_Set_Beam_End`
  (params (Location :type "Vector Structure"))
  ;[1 1 1] RPC
  (`NiagaraComponent.SetVariableVec3` (`self.NS_Laser1`) "Beam End" Location))

(event `Server_Deactivate_Laser`
  ;[1 1 1] RPC
  (`self.Multi_Deactivate_Laser`))

(event `Multi_Deactivate_Laser`
  ;[1 1 1] RPC
  (`ActorComponent.Deactivate` (`self.NS_Laser1`)))

(event `Server_Activate_Vacuum`
  ;[1 1 1] RPC
  (`self.Multi_Activate_Vacuum`))

(event `Server_Deactivate_Vacuum`
  ;[1 1 1] RPC
  (`self.Multi_Deactivate_Vacuum`))

(event `self.D_Capsule.OnComponentBeginOverlap`
  (params (OverlappedComponent :type "PrimitiveComponent Object Reference") (OtherActor :type "Actor Object Reference") (OtherComp :type "PrimitiveComponent Object Reference") (OtherBodyIndex :type Integer) (bFromSweep :type Boolean) (SweepResult :type "HitResult Structure (by ref)"))
  ;[1 1 1] 드릴 데미지
  (`self.Server_Drill_Damage`))

(event `Multi_Activate_Vacuum`
  ;[1 1 1] RPC
  (`ActorComponent.Activate` (`self.NS_Spiral`) false))

(event `Multi_Deactivate_Vacuum`
  ;[1 1 1] RPC
  (`ActorComponent.Deactivate` (`self.NS_Spiral`)))

(event `Server_Drill_Damage`
  (bind __outtooldamage (`self._OutToolDamage`))
  (bind _returnvalue (`SceneComponent.K2_GetComponentLocation` (`self.D_Capsule`)))
  ;[1 1 1] 드릴 데미지
  (if (not (`self.bIsCollectingDrill`))
    (bind _asbody_base (cast `BodyBase` (stale `self.D_Capsule.OnComponentBeginOverlap` OtherActor))
      (:`then`
        (`BodyBase.Damage_Body` _asbody_base __outtooldamage _returnvalue))
      (:`CastFailed`
        (bind _aspanel_base (cast `PanelBase` (stale `self.D_Capsule.OnComponentBeginOverlap` OtherActor))
          (:`then`
            (`PanelBase.Damage_Panel` _aspanel_base __outtooldamage _returnvalue))
          (:`CastFailed`
            (bind _asattachment_base (cast `Attachment_Base` (stale `self.D_Capsule.OnComponentBeginOverlap` OtherActor)))
            (`Attachment_Base.Damage_Attachment` _asattachment_base __outtooldamage _returnvalue)))))))

(event `Vacuum_On_Server`
  (bind _collect_target (`self.Collect_Target`))
  (bind _mesh (`Collectable_base.Mesh` _collect_target))
  (bind _returnvalue (- (`SceneComponent.K2_GetComponentLocation` (`self.V_Scene`)) (`SceneComponent.K2_GetComponentLocation` _mesh)))
  ;[1 1 1] 흡입
  (set `self.bVacuum` true)
  (`self.Multi_Activate_Vacuum`)
  (`/Engine/EditorBlueprintResources/StandardMacros.IsValid` _collect_target
    (:`Is Valid`
      (`PrimitiveComponent.AddForce` _mesh (* (`KismetMathLibrary.Normal` _returnvalue) (/ (`self.MaxForce`) (`KismetMathLibrary.Square` (+ (/ (`KismetMathLibrary.VSize` _returnvalue) (`self.CL`)) 1.0)))) "None" false))))

(event `Vacuum_Off_Server`
  ;[1 1 1] 흡입
  (set `self.bVacuum` false)
  (`self.Multi_Deactivate_Vacuum`))

(event `Drill_On_Server`
  (bind _d_scene (`self.D_Scene`))
  ;[1 1 1] 드릴 데미지
  (`self.Rotate_Drill`)
  (if (not (`self.bThrown`))
    (set `self.bThrown` true)
    (bind _output_get (set `self.Pre_Drill_Loc` (`SceneComponent.K2_GetComponentLocation` _d_scene)))
    (`SceneComponent.SetVisibility` (`self.Cable`) true false)
    (bind (_direction _shoot) (`Timeline|Timeline_3` :!via `PlayFromStart`)
      (:`Update`
        (`SceneComponent.K2_SetWorldLocation` (`self.D_Drill`) (`KismetMathLibrary.VLerp` (`self.Pre_Drill_Loc`) (+ _output_get (* (`SceneComponent.GetForwardVector` _d_scene) 5000.0)) _shoot) true false))
      (:`Finished`
        (`self.Drill_Off_Server`)))))

(event `Drill_Off_Server`
  (bind _d_drill (`self.D_Drill`))
  ;[1 1 1] 드릴 데미지
  (set `self.bIsCollectingDrill` true)
  (bind (_direction _shoot) (`Timeline|Timeline_2` :!via `PlayFromStart`)
    (:`Update`
      (`SceneComponent.K2_SetWorldLocation` _d_drill (`KismetMathLibrary.VLerp` (`SceneComponent.K2_GetComponentLocation` _d_drill) (`SceneComponent.K2_GetComponentLocation` (`self.D_Scene`)) _shoot) false false)
      (if (>= _shoot 0.2)
        (`SceneComponent.SetVisibility` (`self.Cable`) false false)))
    (:`Finished`
      (set `self.bThrown` false)
      (set `self.bIsCollectingDrill` false))))

(fn `DisembarkCharacter`
  (bind _pre_player (`self.Pre_Player`))
  (bind _wbp_collectpanel (`self.Wbp_CollectPanel`))
  (`Controller.Possess` (`self.GetController`) _pre_player)
  (`/Engine/EditorBlueprintResources/StandardMacros.IsValid` _pre_player
    (:`Is Valid`
      (`PSJ_Character.Client_RestoreInputRPC` _pre_player)
      (`/Engine/EditorBlueprintResources/StandardMacros.IsValid` _wbp_collectpanel
        (:`Is Valid`
          (`Widget.RemoveFromParent` _wbp_collectpanel))))))

(fn `UserConstructionScript`)