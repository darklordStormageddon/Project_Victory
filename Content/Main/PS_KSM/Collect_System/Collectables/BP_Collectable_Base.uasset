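; BP_Collectable_Base is the base collectable ore actor, identified by its OreType.
; On BeginPlay it writes the type into its WBP_Floating_Text name widget.
; Highlight events toggle an outline overlay material on the mesh and the name widget's visibility.
; Collect_Ore looks up the type in OreDatatable and, if found, adds one of that element to the game state, without destroying the actor.
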(event `self.ReceiveBeginPlay`
  (bind _aswbp_floating_text (cast `/Game/Main/PS_KSM/Collect_System/Collectables/WBP_Floating_Text` (`WidgetComponent.GetWidget` (`self.Name`))))
  (set `TextBlock.Text` (`KismetTextLibrary.Conv_StringToText` (`self.Ore_Type`)) (`/Game/Main/PS_KSM/Collect_System/Collectables/WBP_Floating_Text.Element_Name` _aswbp_floating_text)))

(event `Enable Highlight`
  (`MeshComponent.SetOverlayMaterial` (`self.Mesh`) "/Game/Main/PS_KSM/Collect_System/Collectables/M_Outline.M_Outline")
  (`SceneComponent.SetVisibility` (`self.Name`) true false))

(event `Disable Highlight`
  (`MeshComponent.SetOverlayMaterial` (`self.Mesh`) null)
  (`SceneComponent.SetVisibility` (`self.Name`) false false))

(event `Collect_Ore`
  (bind _returnvalue (`|GetDataTableRow` (`self.Ore_Datatable`) (`KismetStringLibrary.Conv_StringToName` (`self.Ore_Type`)))
    (:`then`
      (`self.Add_Elem_To_GameState` (`.Name_10_429A16CA43C610F0E61FF89ECA985776` (break `/Game/Main/PS_KSM/Collect_System/Collectables/DS_Collectable` _returnvalue)) 1))))

(fn `UserConstructionScript`)