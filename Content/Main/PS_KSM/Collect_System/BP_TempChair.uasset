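; BP_TempChair is an interactable chair actor that switches the player from the character to the collection panel.
; Its sphere overlap stores an entering PSJ_Character and enables input on the chair, then clears the reference and disables input on exit.
; IA_Interact finds BP_Collect_Panel in the level, passes it the stored character as PrePlayer, and has player controller 0 possess the panel.
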(event `self.ReceiveBeginPlay`)

(event `self.Sphere.OnComponentBeginOverlap`
  (params (OverlappedComponent :type "PrimitiveComponent Object Reference") (OtherActor :type "Actor Object Reference") (OtherComp :type "PrimitiveComponent Object Reference") (OtherBodyIndex :type Integer) (bFromSweep :type Boolean) (SweepResult :type "HitResult Structure (by ref)"))
  (bind _aspsj_character (cast `PSJ_Character` OtherActor))
  (`/Engine/EditorBlueprintResources/StandardMacros.IsValid` (`self.PSJ Character`)
    (:`Is Not Valid`
      (set `self.PSJ Character` _aspsj_character)
      (`self.EnableInput` (`GameplayStatics.GetPlayerController` 0)))))

(event `self.Sphere.OnComponentEndOverlap`
  (params (OverlappedComponent :type "PrimitiveComponent Object Reference") (OtherActor :type "Actor Object Reference") (OtherComp :type "PrimitiveComponent Object Reference") (OtherBodyIndex :type Integer))
  (cast `PSJ_Character` OtherActor)
  (set `self.PSJ Character` null)
  (`self.DisableInput` (`GameplayStatics.GetPlayerController` 0)))

(event `EnhancedInput|/Game/Main/PS_JHS/Input/IA/IA_Interact`
  (params (ActionValue :type Boolean) (ElapsedSeconds :type "Float (double-precision)") (TriggeredSeconds :type "Float (double-precision)") (InputAction :type "InputAction Object Reference" :default "/Game/Main/PS_JHS/Input/IA/IA_Interact.IA_Interact"))
  (:`Triggered`
    (bind _returnvalue (`GameplayStatics.GetActorOfClass` "/Game/Main/PS_KSM/Collect_System/BP_Collect_Panel.BP_Collect_Panel_C"))
    (set `/Game/Main/PS_KSM/Collect_System/BP_Collect_Panel.Pre_Player` (`self.PSJ Character`) _returnvalue)
    (`Controller.Possess` (`GameplayStatics.GetPlayerController` 0) _returnvalue)))

(fn `UserConstructionScript`)