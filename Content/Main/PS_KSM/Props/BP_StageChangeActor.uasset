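; Stage-change actor that moves all MyPSJ_Character players between the lobby spaceship and the stage.
; Starting a stage teleports each to a random BP_StartLoc, unloads the sublevel through the game instance and turns audio on.
; Returning loads the sublevel and plays a timed movie widget with input and audio off.
; The game instance's load-complete callback gathers BP_EndLoc positions and, after a delay, teleports characters to random ones.
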(event `self.ReceiveBeginPlay`
  (`|ExecutionSequence`
    (:`then_0`
      (bind _asbp_my_game_instance (cast `/Game/Main/PS_KSM/GameSettings/BP_MyGameInstance` (`GameplayStatics.GetGameInstance`)))
      (bind _output_get (set `self.As BP My Game Instance` _asbp_my_game_instance))
      (add `/Game/Main/PS_KSM/GameSettings/BP_MyGameInstance.LevelLoadComlete` _output_get (delegate `Load Complete`)))
    (:`then_1`
      (bind _outactors (`GameplayStatics.GetAllActorsOfClass` "/Game/Main/PS_KSM/Props/BP_StartLoc.BP_StartLoc_C"))
      (for _array_element _outactors
        (`KismetArrayLibrary.Array_Add` (`self.StartLoc`) _array_element)))))

(event `Load Complete`
  (bind _outactors (`GameplayStatics.GetAllActorsOfClass` "/Game/Main/PS_KSM/Props/BP_EndLoc.BP_EndLoc_C"))
  (for _array_element _outactors
    (`KismetArrayLibrary.Array_Add` (`self.EndLoc`) (`self.K2_GetActorLocation` _array_element)))
  (`self.Teleport`))

(event `Teleport`
  (if (`self.bIsStarting`)
    (bind _outactors (`GameplayStatics.GetAllActorsOfClass` "/Game/Main/PS_PSJ/Blueprint/PlayerCharacter/MyPSJ_Character.MyPSJ_Character_C"))
    (for _array_element _outactors
      (`/Game/Main/PS_PSJ/Blueprint/PlayerCharacter/MyPSJ_Character.Teleport_Location` _array_element (`self.K2_GetActorLocation` (`KismetArrayLibrary.Array_Random` (`self.StartLoc`)))))
    (else
      (`KismetSystemLibrary.Delay` 1.0)
      (bind _outactors_2 (`GameplayStatics.GetAllActorsOfClass` "/Game/Main/PS_PSJ/Blueprint/PlayerCharacter/MyPSJ_Character.MyPSJ_Character_C"))
      (for _array_element_2 _outactors_2
        (`PSJ_Character.TeleportToSpaceship` _array_element_2 (`KismetArrayLibrary.Array_Random` (`self.EndLoc`)) (`KismetMathLibrary.MakeRotator` 0.0))))))

(event `self.OnStartStage`
  (params (Event :type "EventOnStartStage Object Reference"))
  (`self.Start Stage Implementation`))

(event `self.OnMoveToLobby`
  (params (Event :type "EventOnToLobby Object Reference"))
  (`self.MoveToLobby_Implement`))

(event `MoveToLobby_Implement`
  (`|ExecutionSequence`
    (:`then_0`
      (`/Game/Main/PS_KSM/GameSettings/BP_MyGameInstance.Load Sublevel` (`self.As BP My Game Instance`))
      (set `self.bIsStarting` false))
    (:`then_1`
      (`self.Multi_Play_Movie`))))

(event `Multi_Activate_Sound`
  (`ActorComponent.Activate` (`self.Audio`) true))

(event `Multi_Deactivate_Sound`
  (`ActorComponent.Deactivate` (`self.Audio`)))

(event `Start Stage Implementation`
  (`KismetSystemLibrary.Delay` 0.2)
  (set `self.bIsStarting` true)
  (`self.Teleport`)
  (`/Game/Main/PS_KSM/GameSettings/BP_MyGameInstance.Unload Sublevel` (`self.As BP My Game Instance`))
  (`self.Multi_Activate_Sound`))

(event `Multi_Play_Movie`
  (bind _returnvalue (`GameplayStatics.GetPlayerController` 0))
  (bind _returnvalue_2 (`GameplayStatics.GetPlayerController` 0))
  (`self.Multi_Deactivate_Sound`)
  (`self.DisableInput` (`Controller.K2_GetPawn` _returnvalue) _returnvalue)
  (bind _returnvalue_3 (`|CreateWidget` "/Game/Main/PS_KSM/UI/WBP_MovieRenderer.WBP_MovieRenderer_C" _returnvalue))
  (bind _output_get (set `self.WBP_Movie` _returnvalue_3))
  (`UserWidget.AddToViewport` _output_get 0)
  (`KismetSystemLibrary.Delay` 7.0)
  (`Widget.RemoveFromParent` (`self.WBP_Movie`))
  (`self.EnableInput` (`Controller.K2_GetPawn` _returnvalue_2) _returnvalue_2)
  (`self.Multi_Activate_Sound`))

(fn `UserConstructionScript`)