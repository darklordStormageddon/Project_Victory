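; Destructible satellite connector that detaches its attachment when its health runs out.
; On BeginPlay the authority applies an outline overlay and binds the health component's death event.
; On death, if the attachment is valid, it broadcasts detachment, spawns an explosion effect and destroys itself.
; The last Connector_Base in the world, found by a global actor count rather than per satellite, first tells its satellite the body can be destroyed.
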(event `self.ReceiveBeginPlay`
  (`/Engine/EditorBlueprintResources/ActorMacros.Switch Has Authority`
    (:`Authority`
      (`MeshComponent.SetOverlayMaterial` (`self.StaticMesh`) "/Game/Main/PS_KSM/Collect_System/Collectables/M_Outline2.M_Outline2")
      (add `HealthComponent.OnDeath` (`self.HealthComp`) (delegate `Broadcast_Destruction`)))))

(event `Broadcast_Destruction`
  (bind _attachment (`self.Attachment`))
  (`/Engine/EditorBlueprintResources/StandardMacros.IsValid` _attachment
    (:`Is Valid`
      (`Attachment_Base.Broadcast_Attachment_Detachment` _attachment)
      (`self.Destruct`))))

(event `Destruct`
  (bind _asbp_satellite_base (cast `/Game/Main/PS_KSM/Sattelites/BP_Satellite_Base` (`self.Attached_Satellite`)))
  (bind _outactors (`GameplayStatics.GetAllActorsOfClass` "/Script/TeamSpaceProject.Connector_Base"))
  (if (== (`KismetArrayLibrary.Array_Length` _outactors) 1)
    (`/Game/Main/PS_KSM/Sattelites/BP_Satellite_Base.CanDestroyBody` _asbp_satellite_base))
  (`NiagaraFunctionLibrary.SpawnSystemAtLocation` "/Game/Main/PS_KSM/Effects/NS_Explode.NS_Explode" (`self.K2_GetActorLocation`))
  (`self.K2_DestroyActor`))

(fn `Damage_Triggered`
  (returns (ReturnValue :type Boolean))
  (return false))

(fn `UserConstructionScript`)