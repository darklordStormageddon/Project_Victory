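; BP_Panel is a destructible satellite panel that can detach and fall, or break apart.
; Detachment events detach its root and enable physics on the geometry collection and box, then allow damage.
; HealthComponent death spawns a master field and crumbles the Chaos cluster, destroying both field and panel after a short delay.
; A separate Impulse event applies a strain field through that master field at the panel's location.
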(event `self.ReceiveBeginPlay`
  (bind _returnvalue (`GameplayStatics.GetActorOfClass` "/Script/ChaosCaching.ChaosCacheManager"))
  (set `self.CCM` _returnvalue)
  (add `self.OnDetached` (delegate `Broadcast_Detachment`))
  (add `HealthComponent.OnDeath` (`self.HealthComponent`) (delegate `Broadcast_Destruction`)))

(event `Explode`
  (bind _returnvalue (`|SpawnActorFromClass` "/Engine/EditorResources/FieldNodes/FS_MasterField.FS_MasterField_C" (`SceneComponent.K2_GetComponentToWorld` (`self.Scene`)) "AlwaysSpawn" "MultiplyWithRoot" null null))
  (set `self.MF` _returnvalue)
  (`GeometryCollectionComponent.CrumbleCluster` (`self.BP_Panel_GeometryCollection`) 0))

(event `Broadcast_Destruction`
  (`self.Destruct_Panel`))

(event `Broadcast_Detachment`
  (`self.Simulate_Physics`))

(event `Impulse`
  (bind _mf (`self.MF`))
  (bind _returnvalue (`SceneComponent.K2_GetComponentLocation` (`self.Scene`)))
  (set `/Engine/EditorResources/FieldNodes/FS_MasterField.worldLocation` _returnvalue _mf)
  (`FieldSystemComponent.ApplyStrainField` (`FieldSystemActor.FieldSystemComponent` _mf) true _returnvalue 5.0 10000.0 0))

(event `Destruct_Panel`
  (bind _bp_panel_geometrycollection (`self.BP_Panel_GeometryCollection`))
  ;[1 1 1] 파괴살
  (`/Engine/EditorBlueprintResources/StandardMacros.IsValid` _bp_panel_geometrycollection
    (:`Is Valid`
      (set `PrimitiveComponent.bApplyImpulseOnDamage` true _bp_panel_geometrycollection)
      (`self.Explode`)
      (`KismetSystemLibrary.Delay` 3.0)
      (`self.K2_DestroyActor` (`self.MF`))
      (`self.K2_DestroyActor`))))

(event `Simulate_Physics`
  ;[1 1 1] 물리 on(떨어짐)
  (`SceneComponent.K2_DetachFromComponent` (`self.DefaultSceneRoot`) "KeepWorld" "KeepWorld" "KeepWorld" true)
  (`PrimitiveComponent.SetSimulatePhysics` (`self.BP_Panel_GeometryCollection`) true)
  (`PrimitiveComponent.SetSimulatePhysics` (`self.Box`) true)
  (set `self.bCanDamage` true))

(fn `UserConstructionScript`)