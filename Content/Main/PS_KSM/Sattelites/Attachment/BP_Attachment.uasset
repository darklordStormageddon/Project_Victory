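; Destructible satellite attachment that releases contained actors when destroyed, with detachment and death events bound through server and multicast setup events.
; On detachment it simulates physics on its capsule with an impulse and enables damage.
; On death it spawns unfinished Containings entries on authority, spawns a master field, crumbles its geometry collection, then removes itself after a delay.
; CanBurst is cleared before Burst runs, so that path skips the explosion Niagara effect.
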(event `self.ReceiveBeginPlay`
  (`/Engine/EditorBlueprintResources/ActorMacros.Switch Has Authority`
    (:`Authority`
      (`self.Server_Setup`))))

(event `Server_Setup`
  (`self.Multi_Setup`))

(event `Multi_Setup`
  (add `self.OnDetached` (delegate `Broadcast Detachment`))
  (add `HealthComponent.OnDeath` (`self.HealthComp`) (delegate `Broadcast Destruction`)))

(event `Server_Destruct`
  (`self.Destruct_Attachment`))

(event `Break`
  ;[1 1 1] 부수기
  (bind _returnvalue (`|SpawnActorFromClass` "/Game/Main/PS_KSM/Sattelites/MF_MasterField.MF_MasterField_C" (`SceneComponent.K2_GetComponentToWorld` (`self.Scene`)) "AlwaysSpawn" "MultiplyWithRoot" null null))
  (set `self.MF` _returnvalue)
  (`GeometryCollectionComponent.CrumbleCluster` (`self.BP_Attachment2_GeometryCollection`) 0))

(event `Broadcast Destruction`
  (`self.Server_Destruct`))

(event `Broadcast Detachment`
  (`self.Server_Simulate_Physics`))

(event `Destruct_Attachment`
  (bind _bp_attachment2_geometrycollection (`self.BP_Attachment2_GeometryCollection`))
  ;[1 1 1] 파괴살
  (`/Engine/EditorBlueprintResources/StandardMacros.IsValid` _bp_attachment2_geometrycollection
    (:`Is Valid`
      (`self.Spawn_Elements`)
      (set `self.bCanBurst` false)
      (`PrimitiveComponent.SetSimulatePhysics` _bp_attachment2_geometrycollection true)
      (set `PrimitiveComponent.bApplyImpulseOnDamage` true _bp_attachment2_geometrycollection)
      (`self.Break`)
      (`self.Burst`)
      (`KismetSystemLibrary.Delay` 3.0)
      (`self.K2_DestroyActor` (`self.MF`))
      (`ActorComponent.Deactivate` (`self.BP_Attachment2_GeometryCollection`))
      (`self.K2_DestroyActor`))))

(event `Spawn_Elements`
  ;[1 1 1] 원소 스폰
  (`/Engine/EditorBlueprintResources/ActorMacros.Switch Has Authority`
    (:`Authority`
      (for (_array_element _array_index) (`self.Containings`)
        (bind (_name _num _bspawn_finished) (break `Elem_Set` _array_element))
        (if (not _bspawn_finished)
          (for _ (range _num)
            (`|SpawnActorFromClass` _name (`KismetMathLibrary.MakeTransform` (`self.Spawn_Location`)) "AdjustIfPossibleButAlwaysSpawn" "MultiplyWithRoot" null null))
          (`self.Set_Spawn_Finished` _array_index))))))

(event `Burst`
  (if (`self.bCanBurst`)
    (`NiagaraFunctionLibrary.SpawnSystemAtLocation` "/Game/Main/PS_KSM/Effects/NS_Explode.NS_Explode" (`self.K2_GetActorLocation`))))

(event `Simulate_Physics`
  (bind _capsule (`self.Capsule`))
  ;[1 1 1] 물리 키기(접착부 없어졌을때)
  (`SceneComponent.K2_DetachFromComponent` (`self.DefaultSceneRoot`) "KeepWorld" "KeepWorld" "KeepWorld" true)
  (`PrimitiveComponent.SetSimulatePhysics` _capsule true)
  (`PrimitiveComponent.AddImpulseAtLocation` _capsule (800.0 800.0 800.0) (`SceneComponent.K2_GetComponentLocation` (`self.BP_Attachment2_GeometryCollection`)) "None")
  (set `self.bCanDamage` true))

(event `Server_Simulate_Physics`
  (`self.Simulate_Physics`))

(event `Impulse`
  (bind _mf (`self.MF`))
  (bind _returnvalue (`SceneComponent.K2_GetComponentLocation` (`self.Scene`)))
  (set `/Engine/EditorResources/FieldNodes/FS_MasterField.worldLocation` _returnvalue _mf)
  (`FieldSystemComponent.ApplyStrainField` (`FieldSystemActor.FieldSystemComponent` _mf) true _returnvalue 5.0 10000.0 0))

(fn `UserConstructionScript`)