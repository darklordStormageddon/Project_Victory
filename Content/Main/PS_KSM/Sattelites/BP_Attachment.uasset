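; Destructible satellite attachment that breaks loose and shatters, built on a Chaos Geometry Collection.
; On detachment it leaves its parent, enables physics on the collection and capsule, and becomes damageable.
; Health component death enables impulse on damage, spawns a master field actor and crumbles the cluster, then destroys field and attachment after a delay.
; A separate Impulse event applies a strain field through that master field, with no caller in this graph.
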(event `self.ReceiveBeginPlay`
  (bind _returnvalue (`GameplayStatics.GetActorOfClass` "/Script/ChaosCaching.ChaosCacheManager"))
  (set `self.CCM` _returnvalue)
  (add `self.OnDetached` (delegate `Broadcast_Detachement`))
  (add `HealthComponent.OnDeath` (`self.HealthComp`) (delegate `Broadcast_Destruction`)))

(event `Broadcast_Destruction`
  (`self.Destruct_Attachment`))

(event `Broadcast_Detachement`
  (`self.Simulate_Physics`))

(event `Break`
  (bind _returnvalue (`|SpawnActorFromClass` "/Engine/EditorResources/FieldNodes/FS_MasterField.FS_MasterField_C" (`SceneComponent.K2_GetComponentToWorld` (`self.Scene`)) "AlwaysSpawn" "MultiplyWithRoot" null null))
  (set `self.MF` _returnvalue)
  (`GeometryCollectionComponent.CrumbleCluster` (`self.BP_Attachment2_GeometryCollection`) 0))

(event `Destruct_Attachment`
  (bind _bp_attachment2_geometrycollection (`self.BP_Attachment2_GeometryCollection`))
  ;[1 1 1] 파괴살
  (`/Engine/EditorBlueprintResources/StandardMacros.IsValid` _bp_attachment2_geometrycollection
    (:`Is Valid`
      (set `PrimitiveComponent.bApplyImpulseOnDamage` true _bp_attachment2_geometrycollection)
      (`self.Break`)
      (`KismetSystemLibrary.Delay` 3.0)
      (`self.K2_DestroyActor` (`self.MF`))
      (`self.K2_DestroyActor`))))

(event `Simulate_Physics`
  ;[1 1 1] 물리 키기(접착부 없어졌을때)
  (`SceneComponent.K2_DetachFromComponent` (`self.DefaultSceneRoot`) "KeepWorld" "KeepWorld" "KeepWorld" true)
  (`PrimitiveComponent.SetSimulatePhysics` (`self.BP_Attachment2_GeometryCollection`) true)
  (`PrimitiveComponent.SetSimulatePhysics` (`self.Capsule`) true)
  (set `self.bCanDamage` true))

(event `Impulse`
  (bind _mf (`self.MF`))
  (bind _returnvalue (`SceneComponent.K2_GetComponentLocation` (`self.Scene`)))
  (set `/Engine/EditorResources/FieldNodes/FS_MasterField.worldLocation` _returnvalue _mf)
  (`FieldSystemComponent.ApplyStrainField` (`FieldSystemActor.FieldSystemComponent` _mf) true _returnvalue 5.0 10000.0 0))

(fn `UserConstructionScript`)