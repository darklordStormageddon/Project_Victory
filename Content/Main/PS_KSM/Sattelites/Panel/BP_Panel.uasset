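; Destructible satellite panel that falls when detached and shatters into the items it contains when its health runs out.
; Detach and death delegates feed Server events that enable box physics with an impulse and damageability, or trigger destruction.
; Destruction spawns Containings on authority, crumbles the Geometry Collection alongside a temporary master field, then destroys the actor after a delay.
; CanBurst is cleared before Burst, so that path skips the explosion Niagara effect.
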(event `Server_Setup`
  (`self.Multi_Setup`))

(event `self.ReceiveBeginPlay`
  (`self.Server_Setup`))

(event `Multi_Setup`
  (add `self.OnDetached` (delegate `Broadcast Detachment`))
  (add `HealthComponent.OnDeath` (`self.HealthComponent`) (delegate `Broadcast Destruction`)))

(event `Break`
  (bind _returnvalue (`|SpawnActorFromClass` "/Game/Main/PS_KSM/Sattelites/MF_MasterField.MF_MasterField_C" (`SceneComponent.K2_GetComponentToWorld` (`self.Scene`)) "AlwaysSpawn" "MultiplyWithRoot" null null))
  (set `self.MF` _returnvalue)
  (`GeometryCollectionComponent.CrumbleCluster` (`self.BP_Panel_GeometryCollection`) 0))

(event `Broadcast Destruction`
  (`self.Server_Destruct`))

(event `Broadcast Detachment`
  (`self.Server_Simulate_Physics`))

(event `Server_Destruct`
  (`self.Destruct_Panel`))

(event `Spawn_Elements`
  ;[1 1 1] 원소 스폰
  (`/Engine/EditorBlueprintResources/ActorMacros.Switch Has Authority`
    (:`Authority`
      (for (_array_element _array_index) (`self.Containings`)
        (bind (_name _num _bspawn_finished) (break `Elem_Set` _array_element))
        (if (not _bspawn_finished)
          (for _ (range _num)
            (`|SpawnActorFromClass` _name (`KismetMathLibrary.MakeTransform` (`self.Spawn_Location`)) "AdjustIfPossibleButAlwaysSpawn" "MultiplyWithRoot" null null))
          (`self.Set_Spawn_Finished` _array_index))))))

(event `Destruct_Panel`
  (bind _bp_panel_geometrycollection (`self.BP_Panel_GeometryCollection`))
  ;[1 1 1] 파괴살
  (`/Engine/EditorBlueprintResources/StandardMacros.IsValid` _bp_panel_geometrycollection
    (:`Is Valid`
      (`self.Spawn_Elements`)
      (`PrimitiveComponent.SetSimulatePhysics` _bp_panel_geometrycollection true)
      (set `self.bCanBurst` false)
      (set `PrimitiveComponent.bApplyImpulseOnDamage` true _bp_panel_geometrycollection)
      (`self.Break`)
      (`self.Burst`)
      (`KismetSystemLibrary.Delay` 3.0)
      (`self.K2_DestroyActor` (`self.MF`))
      (`ActorComponent.Deactivate` (`self.BP_Panel_GeometryCollection`))
      (`self.K2_DestroyActor`))))

(event `Server_Simulate_Physics`
  (`self.Simulate_Physics`))

(event `Simulate_Physics`
  (bind _box (`self.Box`))
  ;[1 1 1] 물리 on(떨어짐)
  (`SceneComponent.K2_DetachFromComponent` (`self.DefaultSceneRoot`) "KeepWorld" "KeepWorld" "KeepWorld" true)
  (`PrimitiveComponent.SetSimulatePhysics` _box true)
  (`PrimitiveComponent.AddImpulseAtLocation` _box (800.0 800.0 800.0) (`SceneComponent.K2_GetComponentLocation` (`self.BP_Panel_GeometryCollection`)) "None")
  (set `self.bCanDamage` true))

(event `Burst`
  (if (`self.bCanBurst`)
    (`NiagaraFunctionLibrary.SpawnSystemAtLocation` "/Game/Main/PS_KSM/Effects/NS_Explode.NS_Explode" (`self.K2_GetActorLocation`))))

(event `Impulse`
  (bind _mf (`self.MF`))
  (bind _returnvalue (`SceneComponent.K2_GetComponentLocation` (`self.Scene`)))
  (set `/Engine/EditorResources/FieldNodes/FS_MasterField.worldLocation` _returnvalue _mf)
  (`FieldSystemComponent.ApplyStrainField` (`FieldSystemActor.FieldSystemComponent` _mf) true _returnvalue 5.0 10000.0 0))

(fn `UserConstructionScript`)