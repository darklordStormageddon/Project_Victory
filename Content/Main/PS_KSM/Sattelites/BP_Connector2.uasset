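; BP_Connector2 is a satellite connector that holds a panel and explodes when its health runs out.
; On begin play it applies an outline overlay material and binds health death to broadcasting the panel's detachment, then destroying itself.
; If it is the last Connector_Base actor in the world, it first tells the attached satellite that its body can be destroyed.
; Its DamageTriggered function always returns false.
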(event `self.ReceiveBeginPlay`
  (`MeshComponent.SetOverlayMaterial` (`self.StaticMesh`) "/Game/Main/PS_KSM/Collect_System/Collectables/M_Outline2.M_Outline2")
  (add `HealthComponent.OnDeath` (`self.HealthComp`) (delegate `Detach_Panel`)))

(event `Detach_Panel`
  (bind _panel (`self.Panel`))
  (`/Engine/EditorBlueprintResources/StandardMacros.IsValid` _panel
    (:`Is Valid`
      (`PanelBase.Broadcast_Panel_Detachment` _panel)
      (`self.Destruct`))))

(event `Destruct`
  (bind _asbp_satellite_base (cast `/Game/Main/PS_KSM/Sattelites/BP_Satellite_Base` (`self.Attached_Satellite`)))
  (bind _outactors (`GameplayStatics.GetAllActorsOfClass` "/Script/TeamSpaceProject.Connector_Base"))
  (if (== (`KismetArrayLibrary.Array_Length` _outactors) 1)
    (`/Game/Main/PS_KSM/Sattelites/BP_Satellite_Base.CanDestroyBody` _asbp_satellite_base))
  (`NiagaraFunctionLibrary.SpawnSystemAtLocation` "/Game/Main/PS_KSM/Effects/NS_Explode.NS_Explode" (`self.K2_GetActorLocation`))
  (`self.K2_DestroyActor`))

(fn `Damage_Triggered`
  (returns (ReturnValue :type Boolean))
  (return false))

(fn `UserConstructionScript`
  (`parent.UserConstructionScript`))