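; Temporary player controller that lets the mouse drag a captured physics actor, with look input disabled.
; Left click toggles the IsCaptured flag on CapturedActor, which is assigned outside this graph, and release clears the reference.
; Each tick traces under the cursor and applies a clamped, distance-scaled impulse toward the hit point.
; Within a close radius it instead adds negative doubled velocity, reversing the mesh's motion.
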(event `self.ReceiveBeginPlay`
  (`self.SetIgnoreLookInput` true))

(event `Key|LeftMouseButton`
  (params (Key :type "Key Structure"))
  (bind _capturedactor (`self.CapturedActor`))
  (bind _capturedactor_2 (`self.CapturedActor`))
  (:`Pressed`
    (`/Engine/EditorBlueprintResources/StandardMacros.IsValid` _capturedactor_2
      (:`Is Valid`
        (set `/Game/Main/PS_KSM/BP_Player.bIsCaptured` true _capturedactor))))
  (:`Released`
    (`/Engine/EditorBlueprintResources/StandardMacros.IsValid` _capturedactor_2
      (:`Is Valid`
        (set `/Game/Main/PS_KSM/BP_Player.bIsCaptured` false _capturedactor)
        (set `self.CapturedActor` null)))))

(event `self.ReceiveTick`
  (params (DeltaSeconds :type "Float (single-precision)"))
  (bind _capturedactor (`self.CapturedActor`))
  (bind (_worldlocation _worlddirection) (`self.DeprojectMousePositionToWorld` self))
  (bind _mesh (`Character.Mesh` _capturedactor))
  (bind _outhit (`KismetSystemLibrary.LineTraceSingle` _worldlocation (+ _worldlocation (* _worlddirection 100000.0)) "TraceTypeQuery1" true))
  (`/Engine/EditorBlueprintResources/StandardMacros.IsValid` _capturedactor
    (:`Is Valid`
      (if (`/Game/Main/PS_KSM/BP_Player.bIsCaptured` _capturedactor)
        (bind _returnvalue (- (`.Location` (`GameplayStatics.BreakHitResult` _outhit)) (`SceneComponent.K2_GetComponentLocation` (`Character.Mesh` _capturedactor))))
        (if (>= (`KismetMathLibrary.VSize` _returnvalue) 300.0)
          (`PrimitiveComponent.AddImpulse` _mesh (`KismetMathLibrary.ClampVectorSize` (* _returnvalue 45.0) -30000.0 30000.0) "None" false)
          (else
            (bind _returnvalue_2 (`PrimitiveComponent.GetPhysicsLinearVelocity` _mesh "None"))
            (`PrimitiveComponent.SetPhysicsLinearVelocity` _mesh (* _returnvalue_2 -2.0) true "None")))))))

(fn `UserConstructionScript`)