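; BP_JHSGameMode_Temp is a game mode that teleports joined players' pawns to random start or end locations.
; BeginPlay caches BP_StartLoc positions, while its BP_EndLoc loop stores the game mode's own location instead of each marker's.
; PostLogin records each new player controller.
; Teleport_To_Start and Teleport_To_End move every valid recorded controller's pawn to a random entry from the matching array, without sweeping.
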(event `self.ReceiveBeginPlay`
  (bind _outactors (`GameplayStatics.GetAllActorsOfClass` "/Game/Main/PS_KSM/Props/BP_StartLoc.BP_StartLoc_C"))
  (for _array_element _outactors
    (`KismetArrayLibrary.Array_Add` (`self.StartLoc`) (`self.K2_GetActorLocation` _array_element)))
  (bind _outactors_2 (`GameplayStatics.GetAllActorsOfClass` "/Game/Main/PS_KSM/Props/BP_EndLoc.BP_EndLoc_C"))
  (for _ _outactors_2
    (`KismetArrayLibrary.Array_Add` (`self.EndLoc`) (`self.K2_GetActorLocation`))))

(event `Teleport_To_Start`
  (for _array_element (`self.NewVar`)
    (`/Engine/EditorBlueprintResources/StandardMacros.IsValid` _array_element
      (:`Is Valid`
        (`self.K2_SetActorLocation` (`Controller.K2_GetPawn` _array_element) (`KismetArrayLibrary.Array_Random` (`self.StartLoc`)) false true)))))

(event `self.K2_PostLogin`
  (params (NewPlayer :type "PlayerController Object Reference"))
  (`KismetArrayLibrary.Array_Add` (`self.NewVar`) NewPlayer))

(event `Teleport_To_End`
  (for _array_element (`self.NewVar`)
    (`/Engine/EditorBlueprintResources/StandardMacros.IsValid` _array_element
      (:`Is Valid`
        (`self.K2_SetActorLocation` (`Controller.K2_GetPawn` _array_element) (`KismetArrayLibrary.Array_Random` (`self.EndLoc`)) false true)))))

(fn `UserConstructionScript`)