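; BP_Collect_Chair is an interactable chair actor that hands player control over to the BP_Collect_Panel in the level.
; On BeginPlay it finds and caches the panel.
; A sphere overlap with BP_Player enables the chair's input and shows a WBP_Temp widget, and leaving reverses both.
; Pressing Enter enables input on the panel, makes player controller 0 possess it and removes the widget.
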(event `self.ReceiveBeginPlay`
  (bind _returnvalue (`GameplayStatics.GetActorOfClass` "/Game/Main/PS_KSM/Collect/BP_Collect_Panel.BP_Collect_Panel_C"))
  (set `self.BP_Collect` _returnvalue))

(event `self.Sphere.OnComponentBeginOverlap`
  (params (OverlappedComponent :type "PrimitiveComponent Object Reference") (OtherActor :type "Actor Object Reference") (OtherComp :type "PrimitiveComponent Object Reference") (OtherBodyIndex :type Integer) (bFromSweep :type Boolean) (SweepResult :type "HitResult Structure (by ref)"))
  (cast `/Game/Main/PS_KSM/BP_Player` OtherActor)
  (`self.EnableInput` (`GameplayStatics.GetPlayerController` 0))
  (bind _returnvalue (`|CreateWidget` "/Game/Main/PS_KSM/Collect/WBP_Temp.WBP_Temp_C"))
  (`UserWidget.AddToViewport` _returnvalue 0))

(event `self.Sphere.OnComponentEndOverlap`
  (params (OverlappedComponent :type "PrimitiveComponent Object Reference") (OtherActor :type "Actor Object Reference") (OtherComp :type "PrimitiveComponent Object Reference") (OtherBodyIndex :type Integer))
  (cast `/Game/Main/PS_KSM/BP_Player` OtherActor)
  (`self.DisableInput` (`GameplayStatics.GetPlayerController` 0))
  (`Widget.RemoveFromParent` (stale `self.Sphere.OnComponentBeginOverlap` _returnvalue)))

(event `Key|Enter`
  (params (Key :type "Key Structure"))
  (bind _returnvalue (`GameplayStatics.GetPlayerController` 0))
  (bind _bp_collect (`self.BP_Collect`))
  (:`Pressed`
    (`self.EnableInput` _bp_collect _returnvalue)
    (`Controller.Possess` _returnvalue _bp_collect)
    (`Widget.RemoveFromParent` (stale `self.Sphere.OnComponentBeginOverlap` _returnvalue))))

(fn `UserConstructionScript`)