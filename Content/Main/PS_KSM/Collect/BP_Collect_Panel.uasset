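; BP_Collect_Panel is a possessable pawn that aims a static mesh and fires damaging line traces at connectors, bodies, panels and attachments.
; Look input turns both the controller and the mesh with inverted axes.
; The F action traces forward from the mesh, casts the hit actor to each part base class and calls its damage function, scaled by hit time, so farther hits deal more.
; Debug lines and printouts show hits and remaining health.
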(event `self.ReceivePossessed`
  (params (NewController :type "Controller Object Reference"))
  (bind _asplayer_controller (cast `PlayerController` NewController))
  (`self.EnableInput` _asplayer_controller))

(event `EnhancedInput|/Game/Main/PS_KSM/GameSettings/Input/IA_Look`
  (params (ActionValue :type "Vector2D Structure") (ElapsedSeconds :type "Float (double-precision)") (TriggeredSeconds :type "Float (double-precision)") (InputAction :type "InputAction Object Reference" :default "/Game/Main/PS_KSM/GameSettings/Input/IA_Look.IA_Look"))
  (bind _returnvalue (* ActionValue_X -1.0))
  (bind _returnvalue_2 (* ActionValue_Y -1.0))
  (:`Triggered`
    (`self.AddControllerYawInput` _returnvalue)
    (`self.AddControllerPitchInput` _returnvalue_2)
    (`SceneComponent.K2_AddLocalRotation` (`self.StaticMesh`) (`KismetMathLibrary.MakeRotator` 0.0 _returnvalue_2 _returnvalue) false false)))

(event `EnhancedInput|/Game/Main/PS_KSM/GameSettings/Input/IA_F`
  (params (ActionValue :type Boolean) (ElapsedSeconds :type "Float (double-precision)") (TriggeredSeconds :type "Float (double-precision)") (InputAction :type "InputAction Object Reference" :default "/Game/Main/PS_KSM/GameSettings/Input/IA_F.IA_F"))
  (bind _returnvalue (`SceneComponent.K2_GetComponentLocation` (`self.StaticMesh`)))
  (:`Triggered`
    (bind _outhit (`KismetSystemLibrary.LineTraceSingle` :`Start` _returnvalue :`End` (+ _returnvalue (* (`SceneComponent.GetForwardVector` (`self.StaticMesh`)) 1500.0)) :`TraceChannel` "TraceTypeQuery1" :`DrawDebugType` "ForDuration"))
    (`KismetSystemLibrary.PrintString` (`KismetSystemLibrary.GetDisplayName` (`.HitActor` (`GameplayStatics.BreakHitResult` _outhit))))
    (`|ExecutionSequence`
      (:`then_0`
        (bind _asconnector_base (cast `Connector_Base` (`.HitActor` (`GameplayStatics.BreakHitResult` _outhit))))
        (bind _returnvalue_2 (* (`.Time` (`GameplayStatics.BreakHitResult` _outhit)) 20.0))
        (`Connector_Base.Damage_Connector` _asconnector_base _returnvalue_2)
        (`KismetSystemLibrary.PrintString` (`KismetStringLibrary.Conv_DoubleToString` (`HealthComponent.CurrentHealth` (`Connector_Base.HealthComp` _asconnector_base)))))
      (:`then_1`
        (bind _asbody_base (cast `BodyBase` (`.HitActor` (`GameplayStatics.BreakHitResult` _outhit))))
        (`BodyBase.Damage_Body` _asbody_base _returnvalue_2)
        (`KismetSystemLibrary.PrintString` (`KismetStringLibrary.Conv_DoubleToString` (`HealthComponent.CurrentHealth` (`BodyBase.HealthComp` _asbody_base)))))
      (:`then_2`
        (bind _aspanel_base (cast `PanelBase` (`.HitActor` (`GameplayStatics.BreakHitResult` _outhit))))
        (`PanelBase.Damage_Panel` _aspanel_base _returnvalue_2)
        (`KismetSystemLibrary.PrintString` (`KismetStringLibrary.Conv_DoubleToString` (`HealthComponent.CurrentHealth` (`PanelBase.HealthComponent` _aspanel_base)))))
      (:`then_3`
        (bind _asattachment_base (cast `Attachment_Base` (`.HitActor` (`GameplayStatics.BreakHitResult` _outhit))))
        (`Attachment_Base.Damage_Attachment` _asattachment_base _returnvalue_2)
        (`KismetSystemLibrary.PrintString` (`KismetStringLibrary.Conv_DoubleToString` (`HealthComponent.CurrentHealth` (`Attachment_Base.HealthComp` _asattachment_base))))))))

(fn `UserConstructionScript`)