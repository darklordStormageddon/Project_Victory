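; BP_Static_asteroid is a map actor that represents a static asteroid with a randomized look.
; On BeginPlay it assigns the StaticAsteroid component a random mesh from MeshList.
; It then waits one frame via a zero-length Delay and destroys itself if it overlaps any actor, so asteroids that land on other objects are removed.
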(event `self.ReceiveBeginPlay`
  (bind _meshlist (`self.MeshList`))
  (`StaticMeshComponent.SetStaticMesh` (`self.Static_asteroid`) (`|GetArrayItem` _meshlist (`KismetMathLibrary.RandomIntegerInRange` 0 (`KismetArrayLibrary.Array_LastIndex` _meshlist))))
  (`KismetSystemLibrary.Delay` 0.0)
  (if (> (`KismetArrayLibrary.Array_Length` (`self.GetOverlappingActors` "/Script/Engine.Actor")) 0)
    (`self.K2_DestroyActor`)))

(fn `UserConstructionScript`)