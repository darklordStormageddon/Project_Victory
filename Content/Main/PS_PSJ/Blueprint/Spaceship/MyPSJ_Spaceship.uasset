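; Player spaceship Blueprint that captures satellites with a gravity field.
; Overlapping a satellite with the Gravity component while idle marks it captured and spawns a BP_GravityField attached to that component.
; The gravity input action toggles the field manually; switching it off destroys the field and releases any captured satellite.
; GetGravityLocation exposes the component's world position, and disconnected logic for spawning a collect panel never runs.
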(event `self.ReceiveBeginPlay`)

(event `self.Gravity.OnComponentBeginOverlap`
  (params (OverlappedComponent :type "PrimitiveComponent Object Reference") (OtherActor :type "Actor Object Reference") (OtherComp :type "PrimitiveComponent Object Reference") (OtherBodyIndex :type Integer) (bFromSweep :type Boolean) (SweepResult :type "HitResult Structure (by ref)"))
  (`/Engine/EditorBlueprintResources/StandardMacros.IsValid` (`self.Captured_Satellite`)
    (:`Is Not Valid`
      (if (not (`self.bIsGravityActive`))
        (bind _asbp_satellite_base (cast `/Game/Main/PS_KSM/Sattelites/BP_Satellite_Base` OtherActor))
        (bind _output_get (set `self.Captured_Satellite` _asbp_satellite_base))
        (set `/Game/Main/PS_KSM/Sattelites/BP_Satellite_Base.bIsCaptured` true _output_get)
        (`self.Activate Gravity` (`KismetMathLibrary.MakeTransform` (`SceneComponent.K2_GetComponentLocation` (`self.Gravity`)) (struct) (10.0 10.0 10.0)))))))

(event `Deactivate Gravity`
  (`self.K2_DestroyActor` (`self.Gravity_Field`))
  (set `self.bIsGravityActive` false)
  (set `self.Gravity_Field` null))

(event `Activate Gravity`
  (params (Transform :type "Transform Structure"))
  (bind _returnvalue (`|SpawnActorFromClass` "/Game/Main/PS_KSM/Collect_System/Gravity/BP_GravityField.BP_GravityField_C" Transform "AlwaysSpawn" "MultiplyWithRoot" null self null))
  (bind _output_get (set `self.Gravity_Field` _returnvalue))
  (`self.K2_AttachToComponent` _output_get (`self.Gravity`) "None" "KeepWorld" "KeepWorld" "KeepWorld" true)
  (set `self.bIsGravityActive` true))

(event `EnhancedInput|/Game/Main/PS_PSJ/Blueprint/Spaceship/IA_GravityControl`
  (params (ActionValue :type "Float (double-precision)") (ElapsedSeconds :type "Float (double-precision)") (TriggeredSeconds :type "Float (double-precision)") (InputAction :type "InputAction Object Reference" :default "/Game/Main/PS_PSJ/Blueprint/Spaceship/IA_GravityControl.IA_GravityControl"))
  (bind _captured_satellite (`self.Captured_Satellite`))
  (:`Started`
    (if (`self.bIsGravityActive`)
      (`/Engine/EditorBlueprintResources/StandardMacros.IsValid` (`self.Gravity_Field`)
        (:`Is Valid`
          (`self.Deactivate Gravity`)
          (`/Engine/EditorBlueprintResources/StandardMacros.IsValid` _captured_satellite
            (:`Is Valid`
              (set `/Game/Main/PS_KSM/Sattelites/BP_Satellite_Base.bIsCaptured` false _captured_satellite)
              (set `self.Captured_Satellite` null)))))
      (else
        (`self.Activate Gravity` (`KismetMathLibrary.MakeTransform` (`SceneComponent.K2_GetComponentLocation` (`self.Gravity`)) (struct) (10.0 10.0 10.0)))))))

(fn `GetGravityLocation`
  (returns (GF_Location :type "Vector Structure"))
  (return (`SceneComponent.K2_GetComponentLocation` (`self.Gravity`))))

(fn `UserConstructionScript`)