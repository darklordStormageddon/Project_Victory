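; BP_SpaceShip is a pilotable spaceship with seat trigger volumes for a pilot, a turret and a worker.
; The pilot seat overlap stores the third-person character as PilotPlayer and sets its TargetSpaceship, which clears on exit.
; StartDrive possesses the ship with player 0, adds the IMC_SpaceShip input mapping, then hides, de-collides and attaches the pilot.
; Turret and worker seat overlaps are empty stubs.
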(event `StartDrive`
  (bind _returnvalue (`GameplayStatics.GetPlayerController` 0))
  (bind _pilotplayer (`self.PilotPlayer`))
  (`Controller.Possess` _returnvalue self)
  (message `EnhancedInputSubsystemInterface.AddMappingContext` (pcsubsystem `EnhancedInputLocalPlayerSubsystem` _returnvalue) "/Game/Main/PS_PSJ/IMC_SpaceShip.IMC_SpaceShip" 100 (struct))
  (`self.SetActorEnableCollision` _pilotplayer false)
  (`self.SetActorHiddenInGame` _pilotplayer true)
  (`self.K2_AttachToComponent` _pilotplayer null "None" "KeepRelative" "KeepRelative" "KeepRelative" true))

(event `self.PilotSeatCollision.OnComponentBeginOverlap`
  (params (OverlappedComponent :type "PrimitiveComponent Object Reference") (OtherActor :type "Actor Object Reference") (OtherComp :type "PrimitiveComponent Object Reference") (OtherBodyIndex :type Integer) (bFromSweep :type Boolean) (SweepResult :type "HitResult Structure (by ref)"))
  (bind _asbp_third_person_character (cast `/Game/import/ThirdPerson/Blueprints/BP_ThirdPersonCharacter` OtherActor))
  (set `self.PilotPlayer` _asbp_third_person_character)
  (set `/Game/import/ThirdPerson/Blueprints/BP_ThirdPersonCharacter.TargetSpaceship` self _asbp_third_person_character))

(event `self.PilotSeatCollision.OnComponentEndOverlap`
  (params (OverlappedComponent :type "PrimitiveComponent Object Reference") (OtherActor :type "Actor Object Reference") (OtherComp :type "PrimitiveComponent Object Reference") (OtherBodyIndex :type Integer))
  (bind _asbp_third_person_character (cast `/Game/import/ThirdPerson/Blueprints/BP_ThirdPersonCharacter` OtherActor))
  (set `/Game/import/ThirdPerson/Blueprints/BP_ThirdPersonCharacter.TargetSpaceship` null _asbp_third_person_character))

(event `self.TurretSeatCollision.OnComponentBeginOverlap`
  (params (OverlappedComponent :type "PrimitiveComponent Object Reference") (OtherActor :type "Actor Object Reference") (OtherComp :type "PrimitiveComponent Object Reference") (OtherBodyIndex :type Integer) (bFromSweep :type Boolean) (SweepResult :type "HitResult Structure (by ref)")))

(event `self.TurretSeatCollision.OnComponentEndOverlap`
  (params (OverlappedComponent :type "PrimitiveComponent Object Reference") (OtherActor :type "Actor Object Reference") (OtherComp :type "PrimitiveComponent Object Reference") (OtherBodyIndex :type Integer)))

(event `self.WorkerSeat1Collision.OnComponentBeginOverlap`
  (params (OverlappedComponent :type "PrimitiveComponent Object Reference") (OtherActor :type "Actor Object Reference") (OtherComp :type "PrimitiveComponent Object Reference") (OtherBodyIndex :type Integer) (bFromSweep :type Boolean) (SweepResult :type "HitResult Structure (by ref)")))

(event `self.WorkerSeat1Collision.OnComponentEndOverlap`
  (params (OverlappedComponent :type "PrimitiveComponent Object Reference") (OtherActor :type "Actor Object Reference") (OtherComp :type "PrimitiveComponent Object Reference") (OtherBodyIndex :type Integer)))

(fn `UserConstructionScript`)